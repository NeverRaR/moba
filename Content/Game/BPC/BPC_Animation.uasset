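; BPC_Animation is an actor component that serves animation montages by animation type.
; It converts the type enum to a row name in the AnimTable data table and reads that row's montage array.
; Getter functions return the montage at a given index, the whole array, the last entry or a random entry.
; A missing row yields an empty result, and the component runs no event logic.
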(fn `GetAllAnimByType`
  (params (AnimType :type "/Game/Game/Data/E_AnimationType Enum" :default "NewEnumerator0"))
  (returns (Montage :type "Array of AnimMontage Object Reference"))
  (bind _returnvalue (`|GetDataTableRow` (`self.AnimTable`) (`KismetStringLibrary.Conv_StringToName` (`|GetEnumeratorNameAsString` AnimType)))
    (:`then`
      (return (`.Montage_8_E7A6E2694ABDC171CBF911A559CC2418` (break `/Game/Game/Data/S_Animation` _returnvalue))))
    (:`RowNotFound`
      (return))))

(fn `GetAnimByType`
  (params (AnimType :type "/Game/Game/Data/E_AnimationType Enum" :default "NewEnumerator0") (Index :type Integer))
  (returns (Montage :type "AnimMontage Object Reference"))
  (bind _returnvalue (`|GetDataTableRow` (`self.AnimTable`) (`KismetStringLibrary.Conv_StringToName` (`|GetEnumeratorNameAsString` AnimType)))
    (:`then`
      (return (`|GetArrayItem` (`.Montage_8_E7A6E2694ABDC171CBF911A559CC2418` (break `/Game/Game/Data/S_Animation` _returnvalue)) Index)))
    (:`RowNotFound`
      (return null))))

(fn `GetLastAnimByType`
  (params (AnimType :type "/Game/Game/Data/E_AnimationType Enum" :default "NewEnumerator0"))
  (returns (Montage :type "AnimMontage Object Reference"))
  (bind _montage (`self.GetAllAnimByType` AnimType))
  (return (`|GetArrayItem` _montage (`KismetArrayLibrary.Array_LastIndex` _montage))))

(fn `GetRandomAnimByType`
  (params (AnimType :type "/Game/Game/Data/E_AnimationType Enum" :default "NewEnumerator0"))
  (returns (Montage :type "AnimMontage Object Reference"))
  (bind _montage (`self.GetAllAnimByType` AnimType))
  (return (`|GetArrayItem` _montage (`KismetMathLibrary.RandomIntegerInRange` 0 (`KismetArrayLibrary.Array_LastIndex` _montage)))))