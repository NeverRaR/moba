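; MOBA game mode that spawns and possesses the two players' heroes and handles match end.
; BeginPlay replaces the saved-index server player's pawn with Kuang, then polls until the client controller exists to give it Shinbi on the opposing camp.
; It then counts heroes per camp and adds an unpossessed Kuang if uneven.
; GameOver relays the camp to player HUDs, then opens LoadingMap after a delay.
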(event `self.ReceiveBeginPlay`
  (`|ExecutionSequence`
    (:`then_0`
      (bind _returnvalue (`GameplayStatics.LoadGameFromSlot` "Player0"))
      (bind _asplayer_index_save_data (cast `/Game/Game/Data/PlayerIndexSaveData` _returnvalue))
      (bind _myplayerindex (`/Game/Game/Data/PlayerIndexSaveData.Get` _asplayer_index_save_data))
      (bind _output_get (set `self.ServerIndex` _myplayerindex))
      (bind _returnvalue_2 (`GameplayStatics.GetPlayerCharacter` _output_get))
      (`/Engine/EditorBlueprintResources/StandardMacros.IsValid` _returnvalue_2
        (:`Is Valid`
          (`self.K2_DestroyActor` _returnvalue_2))))
    (:`then_1`
      (bind _returnvalue_3 (`GameplayStatics.LoadGameFromSlot` "Save"))
      (bind _asmy_save_data (cast `/Game/Game/Data/MySaveData` _returnvalue_3))
      (bind _outactors (`GameplayStatics.GetAllActorsOfClass` "/Script/Engine.PlayerStart"))
      (bind _returnvalue_4 (`|SpawnActorFromClass` "/Game/Game/Role/BP_Kuang.BP_Kuang_C" (`self.GetTransform` (`|GetArrayItem` _outactors)) "Undefined" "OverrideRootScale" null null))
      (`CreatureCamp.SetCamp` (`BaseCharacter.CampComp` _returnvalue_4) (`self.Camp1`))
      (`Controller.Possess` (`GameplayStatics.GetPlayerController` (`self.ServerIndex`)) _returnvalue_4)
      (`/Game/Game/Role/BP_Kuang.InitCamp` _returnvalue_4))
    (:`then_2`
      (`KismetSystemLibrary.Delay` 0.2 :!label _label)
      (`/Engine/EditorBlueprintResources/StandardMacros.IsValid` (`GameplayStatics.GetPlayerController` (`self.ClientIndex`))
        (:`Is Valid`
          (bind _returnvalue_5 (`GameplayStatics.LoadGameFromSlot` "Save"))
          (bind _asmy_save_data_2 (cast `/Game/Game/Data/MySaveData` _returnvalue_5))
          (bind _outactors_2 (`GameplayStatics.GetAllActorsOfClass` "/Script/Engine.PlayerStart"))
          (bind _returnvalue_6 (`|SpawnActorFromClass` "/Game/Game/Role/BP_Shinbi.BP_Shinbi_C" (`self.GetTransform` (`|GetArrayItem` _outactors_2)) "Undefined" "OverrideRootScale" null null))
          (`CreatureCamp.SetCamp` (`BaseCharacter.CampComp` _returnvalue_6) (`self.Camp2`))
          (`Controller.Possess` (`GameplayStatics.GetPlayerController` (`self.ClientIndex`)) _returnvalue_6)
          (`/Game/Game/Role/BP_Shinbi.InitCamp` _returnvalue_6)
          (bind _outactors_3 (`GameplayStatics.GetAllActorsOfClass` "/Script/OurMoba.Hero"))
          (for _array_element _outactors_3
            (bind _returnvalue_7 (`CreatureCamp.GetCamp` (`BaseCharacter.CampComp` _array_element)))
            (switch `CharacterCamp` _returnvalue_7
              (:`Dawn`
                (set `self.Dawn` (+ (`self.Dawn`) 1)))
              (:`Dust`
                (set `self.Dust` (+ (`self.Dust`) 1)))))
          (if (>= (`self.Dawn`) (`self.Dust`))
            (if (< (`self.Dust`) (`self.Dawn`))
              (bind _outactors_4 (`GameplayStatics.GetAllActorsOfClass` "/Script/Engine.PlayerStart"))
              (bind _returnvalue_8 (`|SpawnActorFromClass` "/Game/Game/Role/BP_Kuang.BP_Kuang_C" (`self.GetTransform` (`|GetArrayItem` _outactors_4)) "Undefined" "OverrideRootScale" null null))
              (`CreatureCamp.SetCamp` (`BaseCharacter.CampComp` _returnvalue_8) (`self.Camp2`))
              (`/Game/Game/Role/BP_Kuang.InitCamp` _returnvalue_8))
            (else
              (bind _outactors_5 (`GameplayStatics.GetAllActorsOfClass` "/Script/Engine.PlayerStart"))
              (bind _returnvalue_9 (`|SpawnActorFromClass` "/Game/Game/Role/BP_Kuang.BP_Kuang_C" (`self.GetTransform` (`|GetArrayItem` _outactors_5)) "Undefined" "OverrideRootScale" null null))
              (`CreatureCamp.SetCamp` (`BaseCharacter.CampComp` _returnvalue_9) (`self.Camp1`))
              (`/Game/Game/Role/BP_Kuang.InitCamp` _returnvalue_9))))
        (:`Is Not Valid`
          (goto _label))))))

(event `CallGameOver`
  (params (Camp :type "CharacterCamp Enum" :default "Dawn") (Pawn :type "Pawn Object Reference"))
  (bind _asplayer_controller (cast `PlayerController` (`Pawn.GetController` Pawn)))
  (bind _asbp_hud (cast `/Game/Game/UI/BP_GameHUD` (`PlayerController.GetHUD` _asplayer_controller)))
  (`/Game/Game/UI/BP_GameHUD.OnGameOver` _asbp_hud Camp))

(event `self.GameOver`
  (params (Camp :type "CharacterCamp Enum" :default "Dawn"))
  (set `self.Camp` Camp)
  (bind _outactors (`GameplayStatics.GetAllActorsOfClass` "/Script/OurMoba.Hero"))
  (for _array_element _outactors
    (`self.CallGameOver` (`self.Camp`) _array_element))
  (`KismetSystemLibrary.Delay` 5.0)
  (`GameplayStatics.OpenLevel` "LoadingMap"))

(fn `UserConstructionScript`)