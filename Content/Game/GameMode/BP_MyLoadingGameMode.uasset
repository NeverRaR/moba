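; BP_MyLoadingGameMode is a game mode, named for loading, that records the controller ID of joining players.
; On PostLogin it creates a PlayerIndexSaveData object, stores the new player's controller ID and saves it to a slot chosen by a running PlayerIndex.
; Only the first two players are saved, as Player0 and Player1.
; Logic enabling seamless travel outside standalone play is present but never runs.
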(event `self.ReceiveBeginPlay`)

(event `self.K2_PostLogin`
  (params (NewPlayer :type "PlayerController Object Reference"))
  (bind _returnvalue (`GameplayStatics.CreateSaveGameObject` "/Game/Game/Data/PlayerIndexSaveData.PlayerIndexSaveData_C"))
  (`/Game/Game/Data/PlayerIndexSaveData.Set` _returnvalue (`GameplayStatics.GetPlayerControllerID` NewPlayer))
  (switch `int` (`self.PlayerIndex`)
    (:`0`
      (`GameplayStatics.SaveGameToSlot` _returnvalue "Player0"))
    (:`1`
      (`GameplayStatics.SaveGameToSlot` _returnvalue "Player1" 1)))
  (set `self.PlayerIndex` (+ (`self.PlayerIndex`) 1)))

(fn `UserConstructionScript`)