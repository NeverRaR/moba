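; Base AI controller that initializes itself from its controlled pawn and can auto-start that pawn's behavior tree.
; On BeginPlay it polls with short delays until a pawn exists, then caches the pawn and its AIManager component.
; That component supplies the tree and auto-run flag.
; Once a blackboard exists, the skeletal mesh's Ground socket location is stored as InitPoint.
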(event `self.ReceiveTick`
  (params (DeltaSeconds :type "Float (single-precision)")))

(event `self.ReceiveBeginPlay`
  (bind _returnvalue (`self.K2_GetPawn`))
  (bind _aicomp (`self.AIComp`))
  (bind _returnvalue_2 (`AIBlueprintHelperLibrary.GetBlackboard` self))
  (bind _returnvalue_3 (`self.GetComponentByClass` (`self.OwnerPawn`) "/Script/OurMoba.AIManager"))
  (bind _behaviortree (`AIManager.BehaviorTree` _aicomp))
  (`|ExecutionSequence`
    (:`then_0`
      (`/Engine/EditorBlueprintResources/StandardMacros.IsValid` _returnvalue :!label _label
        (:`Is Valid`
          (set `self.OwnerPawn` _returnvalue)
          (set `self.bIsInit` true)
          (`|ExecutionSequence`
            (:`then_0`
              (`/Engine/EditorBlueprintResources/StandardMacros.IsValid` _returnvalue_3
                (:`Is Valid`
                  (set `self.AIComp` _returnvalue_3))))
            (:`then_1`
              (`/Engine/EditorBlueprintResources/StandardMacros.IsValid` _returnvalue_2 :!label _label_2
                (:`Is Valid`
                  (`BlackboardComponent.SetValueAsVector` _returnvalue_2 "InitPoint" (`SceneComponent.GetSocketLocation` (`self.GetComponentByClass` (`self.OwnerPawn`) "/Script/Engine.SkeletalMeshComponent") "Ground")))
                (:`Is Not Valid`
                  (`KismetSystemLibrary.Delay` 0.2)
                  (goto _label_2))))))
        (:`Is Not Valid`
          (`KismetSystemLibrary.Delay` 0.1)
          (goto _label))))
    (:`then_1`
      (if (`self.bIsInit`) :!label _label_3
        (`/Engine/EditorBlueprintResources/StandardMacros.IsValid` _aicomp
          (:`Is Valid`
            (if (`AIManager.bIsAutoRun` _aicomp)
              (`/Engine/EditorBlueprintResources/StandardMacros.IsValid` _behaviortree
                (:`Is Valid`
                  (`self.RunBehaviorTree` _behaviortree))))))
        (else
          (`KismetSystemLibrary.Delay` 0.1)
          (goto _label_3))))))

(fn `UserConstructionScript`)