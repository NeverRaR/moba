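; AI controller for melee minions that manages perception and hate-based attack targeting.
; Init retries until the pawn exists, caches its components, writes the InitPoint blackboard key and runs the AI component's behavior tree when auto-run is set.
; Perceived characters split into friends and enemies, with enemies seeding a hate list that GetAttackTarget weights by distance.
; Death events from minions and turrets prune these lists, while Tick prints the current target.
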(event `self.ReceiveBeginPlay`
  (bind _returnvalue (`self.K2_GetPawn`))
  (bind _aicomp (`self.AIComp`))
  (bind _returnvalue_2 (`AIBlueprintHelperLibrary.GetBlackboard` self))
  (bind _returnvalue_3 (`self.GetComponentByClass` (`self.OwnerPawn`) "/Script/OurMoba.CreatureCamp"))
  (bind _returnvalue_4 (`self.GetComponentByClass` (`self.OwnerPawn`) "/Game/Game/BPC/BPC_AIManager.BPC_AIManager_C"))
  (bind _behaviortree (`/Game/Game/BPC/BPC_AIManager.BehaviorTree` _aicomp))
  (`|ExecutionSequence`
    (:`then_0`
      (`/Engine/EditorBlueprintResources/StandardMacros.IsValid` _returnvalue :!label _label
        (:`Is Valid`
          (set `self.OwnerPawn` _returnvalue)
          (set `self.IsInit` true)
          (`|ExecutionSequence`
            (:`then_0`
              (`/Engine/EditorBlueprintResources/StandardMacros.IsValid` _returnvalue_4
                (:`Is Valid`
                  (set `self.AIComp` _returnvalue_4))))
            (:`then_1`
              (`/Engine/EditorBlueprintResources/StandardMacros.IsValid` _returnvalue_3
                (:`Is Valid`
                  (set `self.CampComp` _returnvalue_3))))
            (:`then_2`
              (`/Engine/EditorBlueprintResources/StandardMacros.IsValid` _returnvalue_2 :!label _label_2
                (:`Is Valid`
                  (`BlackboardComponent.SetValueAsVector` _returnvalue_2 "InitPoint" (`SceneComponent.GetSocketLocation` (`self.GetComponentByClass` (`self.OwnerPawn`) "/Script/Engine.SkeletalMeshComponent") "Ground")))
                (:`Is Not Valid`
                  (`KismetSystemLibrary.Delay` 0.2)
                  (goto _label_2))))))
        (:`Is Not Valid`
          (`KismetSystemLibrary.Delay` 0.1)
          (goto _label))))
    (:`then_1`
      (if (`self.IsInit`) :!label _label_3
        (`/Engine/EditorBlueprintResources/StandardMacros.IsValid` _aicomp
          (:`Is Valid`
            (if (`/Game/Game/BPC/BPC_AIManager.IsAutoRun` _aicomp)
              (`/Engine/EditorBlueprintResources/StandardMacros.IsValid` _behaviortree
                (:`Is Valid`
                  (`self.RunBehaviorTree` _behaviortree))))))
        (else
          (`KismetSystemLibrary.Delay` 0.1)
          (goto _label_3))))))

(event `self.AIPerception.OnPerceptionUpdated`
  (params (UpdatedActors :type "Array of Actor Object Reference (by ref)"))
  (if (`self.IsInit`)
    (for _array_element UpdatedActors
      (`KismetArrayLibrary.Array_AddUnique` (`self.PerceprionActors`) _array_element))
    (bind _issuccessful (`self.CheckAllTarget`))
    (if _issuccessful
      (for _array_element_2 (`self.PerceprionActors`)
        (`/Engine/EditorBlueprintResources/StandardMacros.IsValid` _array_element_2
          (:`Is Valid`
            (bind _asbp_minion_melee (cast `/Game/Game/Role/BP_Minion_Melee` _array_element_2)
              (:`then`
                (add `/Game/Game/Role/BP_Minion_Melee.DP_ActorDeath` _asbp_minion_melee (delegate `OneTargetDeath`)))
              (:`CastFailed`
                (bind _asbp_minion_ranged (cast `/Game/Game/Role/BP_Minion_Ranged` _array_element_2)
                  (:`then`
                    (add `/Game/Game/Role/BP_Minion_Ranged.DP_ActorDeath` _asbp_minion_ranged (delegate `OneTargetDeath`)))
                  (:`CastFailed`
                    (bind _asbp_turret (cast `/Game/Game/Role/BP_Turret` _array_element_2))
                    (add `/Game/Game/Role/BP_Turret.DP_ActorDeath` _asbp_turret (delegate `OneTargetDeath`))))))))))))

(event `self.ReceiveTick`
  (params (DeltaSeconds :type "Float (single-precision)"))
  (bind (_issuccessful _attacktarget) (`self.GetAttackTarget`))
  (`KismetSystemLibrary.PrintString` (`KismetSystemLibrary.GetDisplayName` _attacktarget)))

(event `OneTargetDeath`
  (params (DeathActor :type "Actor Object Reference"))
  (`self.RemoveOneTarget` DeathActor))

(event `self.ClearAttackTarget`
  (bind (_issuccessful _attacktarget) (`self.GetAttackTarget`))
  (`self.RemoveOneTarget` _attacktarget))

(fn `AddHateValue`
  (params (Attacker :type "Actor Object Reference (by ref)") (HateVlaue :type "Float (double-precision)"))
  (returns (IsSuccessful :type Boolean))
  (for (_array_element _array_index) (`self.HateList`)
    (bind (_target _value) (break `/Game/Game/AI/S_HateValue` _array_element))
    (if (== _target Attacker)
      (setmembers `/Game/Game/AI/S_HateValue` :`StructRef` (`|GetArrayItem` (`self.HateList`) _array_index) :`Target` null :`Value` (+ _value HateVlaue)))))

(fn `CheckAllTarget`
  (returns (IsSuccessful :type Boolean))
  (bind _perceprionactors (`self.PerceprionActors`))
  (`/Engine/EditorBlueprintResources/StandardMacros.IsValid` (`self.OwnerPawn`)
    (:`Is Valid`
      (if (`KismetArrayLibrary.Array_IsValidIndex` _perceprionactors)
        (for _array_element _perceprionactors
          (`/Engine/EditorBlueprintResources/StandardMacros.IsValid` _array_element
            (:`Is Valid`
              (bind _asbase_character (cast `BaseCharacter` _array_element))
              (bind _asbase_character_2 (cast `BaseCharacter` (`self.OwnerPawn`)))
              (bind _returnvalue (`BaseCharacter.CheckIsEnemy` _asbase_character_2 _asbase_character))
              (if _returnvalue
                (`KismetArrayLibrary.Array_AddUnique` (`self.Enemys`) _array_element)
                (`self.RefreshHateList` _array_element)
                (else
                  (`KismetArrayLibrary.Array_AddUnique` (`self.Friends`) _array_element))))))
        (return true)))
    (:`Is Not Valid`
      (return false))))

(fn `CheckHateList`
  (params (NewEnemy :type "Actor Object Reference"))
  (returns (IsIncluded :type Boolean))
  (for _array_element (`self.HateList`)
    (if (== (`.Target_2_FA55F19C46C58002A64DF89B8CD9C764` (break `/Game/Game/AI/S_HateValue` _array_element)) NewEnemy)
      (return true)))
  (return false))

(fn `GetAttackTarget`
  (returns (IsSuccessful :type Boolean) (AttackTarget :type "Actor Object Reference") (HateValue :type "Float (double-precision)"))
  (locals (vHitValueByDistance :type "Array of Float (double-precision)") (vMaxIndex :type Integer :default 0))
  (bind (_target _value) (break `/Game/Game/AI/S_HateValue` (`|GetArrayItem` (`self.HateList`) (`local.vMaxIndex`))))
  (`/Engine/EditorBlueprintResources/StandardMacros.IsValid` (`self.OwnerPawn`)
    (:`Is Valid`
      (`KismetArrayLibrary.Array_Clear` (`self.HateListByDistance`))
      (if (`KismetArrayLibrary.Array_IsValidIndex` (`self.HateList`))
        (for _array_element (`self.HateList`)
          (bind (_target_2 _value_2) (break `/Game/Game/AI/S_HateValue` _array_element))
          (`/Engine/EditorBlueprintResources/StandardMacros.IsValid` _target_2
            (:`Is Valid`
              (bind _value_3 (`self.HateValueByDistance` (`self.GetDistanceTo` (`self.OwnerPawn`) _target_2)))
              (bind _returnvalue (* _value_2 _value_3))
              (`KismetArrayLibrary.Array_Add` (`local.vHitValueByDistance`) _returnvalue)
              (`KismetArrayLibrary.Array_AddUnique` (`self.HateListByDistance`) (make `/Game/Game/AI/S_HateValue` _target_2 _returnvalue)))))
        (set `local.vMaxIndex` (`KismetMathLibrary.MaxOfFloatArray` (`local.vHitValueByDistance`)))
        (`/Engine/EditorBlueprintResources/StandardMacros.IsValid` _target
          (:`Is Valid`
            (return true _target _value))
          (:`Is Not Valid`
            (return true null 0.0)))
        (else
          (return false null 0.0))))
    (:`Is Not Valid`
      (return false null 0.0))))

(fn `HateValueByDistance`
  (params (Distance :type "Float (double-precision)"))
  (returns (Value :type "Float (double-precision)"))
  (return (`KismetMathLibrary.SelectFloat` 0.0 (`KismetMathLibrary.Lerp` 2.0 0.1 (`KismetMathLibrary.FClamp` (/ Distance 3000.0))) (> Distance 5000.0))))

(fn `RefreshHateList`
  (params (Enemy :type "Actor Object Reference"))
  (`/Engine/EditorBlueprintResources/StandardMacros.IsValid` Enemy
    (:`Is Valid`
      (if (`KismetArrayLibrary.Array_IsValidIndex` (`self.HateList`))
        (bind _isincluded (`self.CheckHateList` Enemy))
        (if _isincluded
          (return)
          (else
            (`KismetArrayLibrary.Array_Add` (`self.HateList`) (make `/Game/Game/AI/S_HateValue` Enemy 10.0))))
        (else
          (`KismetArrayLibrary.Array_Add` (`self.HateList`) (make `/Game/Game/AI/S_HateValue` Enemy 10.0)))))))

(fn `RemoveOneTarget`
  (params (Target :type "Actor Object Reference"))
  (returns (IsSuccessful :type Boolean))
  (locals (LocalActor :type "Actor Object Reference"))
  (bind _enemys (`self.Enemys`))
  (bind _localactor (`local.LocalActor`))
  (bind _friends (`self.Friends`))
  (bind _localactor_2 (`local.LocalActor`))
  (`/Engine/EditorBlueprintResources/StandardMacros.IsValid` Target
    (:`Is Valid`
      (bind _output_get (set `local.LocalActor` Target))
      (if (`KismetArrayLibrary.Array_Contains` (`self.PerceprionActors`) _output_get)
        (`KismetArrayLibrary.Array_RemoveItem` (`self.PerceprionActors`) (`local.LocalActor`))
        (for _array_element (`self.HateList`)
          (if (== (`.Target_2_FA55F19C46C58002A64DF89B8CD9C764` (break `/Game/Game/AI/S_HateValue` _array_element)) (`local.LocalActor`))
            (`KismetArrayLibrary.Array_RemoveItem` (`self.HateList`) _array_element)))
        (if (`KismetArrayLibrary.Array_Contains` _enemys _localactor)
          (bind _returnvalue (`KismetArrayLibrary.Array_RemoveItem` _enemys _localactor))
          (return _returnvalue)
          (elif (`KismetArrayLibrary.Array_Contains` _friends _localactor_2)
            (bind _returnvalue_2 (`KismetArrayLibrary.Array_RemoveItem` _friends _localactor_2))
            (return _returnvalue_2)
            (else
              (return false))))
        (else
          (return false))))))

(fn `UserConstructionScript`)