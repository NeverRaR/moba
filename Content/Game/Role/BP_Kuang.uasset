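; BP_Kuang is a playable MOBA character with camp, property and skill components.
; Shortly after BeginPlay, a locally controlled player takes Dawn with authority or Dusk otherwise, syncing Dusk through server events.
; Camp-init events teleport the pawn to its camp's start actor.
; Tick feeds health ratio to the KuangHP widget, GameOver forwards the camp to the HUD, and two inputs print skill cooldown and nearby-enemy debug info.
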(event `GameOver`
  (params (Camp :type "CharacterCamp Enum" :default "Dawn"))
  (bind _asbp_moba_controller (cast `/Game/Game/Role/BP_MobaController` (`self.GetController`)))
  (bind _asbp_game_hud (cast `/Game/Game/UI/BP_GameHUD` (`PlayerController.GetHUD` _asbp_moba_controller)))
  (`/Game/Game/UI/BP_GameHUD.OnGameOver` _asbp_game_hud Camp))

(event `ServerSetCamp`
  (params (NewParam :type "CharacterCamp Enum" :default "Dawn"))
  (`CreatureCamp.SetCamp` (`self.CampComp`) NewParam))

(event `self.ReceiveBeginPlay`
  (bind _returnvalue (`self.GetController`))
  (`KismetSystemLibrary.Delay` 0.2)
  (`/Engine/EditorBlueprintResources/StandardMacros.IsValid` _returnvalue
    (:`Is Valid`
      (if (`Controller.IsLocalPlayerController` _returnvalue)
        (if (`self.HasAuthority` _returnvalue)
          (`CreatureCamp.SetCamp` (`self.CampComp`) (`self.Dawn`))
          (`self.InitCamp`)
          (else
            (`CreatureCamp.SetCamp` (`self.CampComp`) (`self.Dusk`))
            (`self.ServerSetCamp` (`self.Dusk`))
            (`self.ServerInitCamp` null)))))))

(event `ServerInitCamp`
  (params (Pawn :type "BaseCharacter Object Reference"))
  (bind _returnvalue (`CreatureCamp.GetCamp` (`self.CampComp`)))
  (switch `CharacterCamp` _returnvalue
    (:`Dawn`
      (bind _outactors (`GameplayStatics.GetAllActorsOfClass` "/Game/Game/Dawn/DawnBeginPlayer.DawnBeginPlayer_C"))
      (bind _output (`|GetArrayItem` _outactors))
      (`/Engine/EditorBlueprintResources/StandardMacros.IsValid` _output
        (:`Is Valid`
          (set `self.OriginLocation` (`self.K2_GetActorLocation` _output)))))
    (:`Dust`
      (bind _outactors_2 (`GameplayStatics.GetAllActorsOfClass` "/Game/Game/Dusk/DuskBeginPlayer.DuskBeginPlayer_C"))
      (bind _output_2 (`|GetArrayItem` _outactors_2))
      (`/Engine/EditorBlueprintResources/StandardMacros.IsValid` _output_2
        (:`Is Valid`
          (set `self.OriginLocation` (`self.K2_GetActorLocation` _output_2))))))
  (`self.K2_SetActorLocation` (`self.OriginLocation`)))

(event `self.BlueprintInitCamp`
  (bind _returnvalue (`CreatureCamp.GetCamp` (`self.CampComp`)))
  (switch `CharacterCamp` _returnvalue
    (:`Dawn`
      (bind _outactors (`GameplayStatics.GetAllActorsOfClass` "/Game/Game/Dawn/DawnBeginPlayer.DawnBeginPlayer_C"))
      (bind _output (`|GetArrayItem` _outactors))
      (`/Engine/EditorBlueprintResources/StandardMacros.IsValid` _output
        (:`Is Valid`
          (set `self.OriginLocation` (`self.K2_GetActorLocation` _output)))))
    (:`Dust`
      (bind _outactors_2 (`GameplayStatics.GetAllActorsOfClass` "/Game/Game/Dusk/DuskBeginPlayer.DuskBeginPlayer_C"))
      (bind _output_2 (`|GetArrayItem` _outactors_2))
      (`/Engine/EditorBlueprintResources/StandardMacros.IsValid` _output_2
        (:`Is Valid`
          (set `self.OriginLocation` (`self.K2_GetActorLocation` _output_2))))))
  (`self.K2_SetActorLocation` (`self.OriginLocation`)))

(event `self.ReceiveTick`
  (params (DeltaSeconds :type "Float (single-precision)"))
  (bind _kuanghp (`self.KuangHP`))
  (bind _propertycomp (`self.PropertyComp`))
  (`|ExecutionSequence`
    (:`then_0`
      (`/Engine/EditorBlueprintResources/StandardMacros.IsValid` _kuanghp
        (:`Is Valid`
          (`|ExecutionSequence`
            (:`then_0`
              (bind _asui_kuang (cast `/Game/Game/UI/UI_Kuang` (`WidgetComponent.GetUserWidgetObject` _kuanghp)))
              (`/Game/Game/UI/UI_Kuang.UpdateKuangHP` _asui_kuang (/ (stale _returnvalue) (`KismetMathLibrary.SelectFloat` 1.0 (stale _returnvalue_2) (== (stale _returnvalue_2) 0.0)))))
            (:`then_1`
              (bind _returnvalue (`CharacterProperty.GetCurHP` _propertycomp))
              (bind _returnvalue_2 (`CharacterProperty.GetCurMaxHP` _propertycomp)))))))))

(event `self.DEBUGprint`
  (params (num :type "Float (single-precision)"))
  (`KismetSystemLibrary.PrintString` (`KismetStringLibrary.Conv_DoubleToString` num)))

(event `InputAction|LevelUp`
  (params (Key :type "Key Structure"))
  (:`Pressed`
    (bind _returnvalue (`Skill.GetSkillCurCD` (`self.SkillComp`) 2))
    (`KismetSystemLibrary.PrintString` (`KismetStringLibrary.Conv_DoubleToString` _returnvalue))))

(event `InputAction|ShowSkillStatus`
  (params (Key :type "Key Structure"))
  (:`Pressed`
    (bind _returnvalue (`self.GetAllEnemysInRadius` 2000.0))
    (`KismetSystemLibrary.PrintString` (`KismetStringLibrary.Conv_IntToString` (`KismetArrayLibrary.Array_Length` _returnvalue)))))

(fn `UserConstructionScript`)