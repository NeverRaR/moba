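; BP_Green is a character Blueprint with a health bar widget and stats supplied by PropertyComp.
; On BeginPlay it sets walk speed from PropertyComp.
; While GreenHP is valid, Tick pushes the HP ratio to its UI_Green widget, guarding against zero max HP, then refreshes cached values, so the bar lags one tick.
; WholeDeath fires the actor-death dispatcher, then destroys the actor.
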(event `self.ReceiveTick`
  (params (DeltaSeconds :type "Float (single-precision)"))
  (bind _greenhp (`self.GreenHP`))
  (bind _propertycomp (`self.PropertyComp`))
  (`|ExecutionSequence`
    (:`then_0`
      (`/Engine/EditorBlueprintResources/StandardMacros.IsValid` _greenhp
        (:`Is Valid`
          (`|ExecutionSequence`
            (:`then_0`
              (bind _asui_green (cast `/Game/Game/UI/UI_Green` (`WidgetComponent.GetUserWidgetObject` _greenhp)))
              (`/Game/Game/UI/UI_Green.UpdateGreenHP` _asui_green (/ (stale _returnvalue) (`KismetMathLibrary.SelectFloat` 1.0 (stale _returnvalue_2) (== (stale _returnvalue_2) 0.0)))))
            (:`then_1`
              (bind _returnvalue (`CharacterProperty.GetCurHP` _propertycomp))
              (bind _returnvalue_2 (`CharacterProperty.GetCurMaxHP` _propertycomp)))))))))

(event `self.DEBUGprint`
  (params (num :type "Float (single-precision)")))

(event `self.SetMoveSpeed`
  (params (CurSpeed :type "Float (single-precision)")))

(event `self.ReceiveBeginPlay`
  (bind _charactermovement (`self.CharacterMovement`))
  (bind _returnvalue (`CharacterProperty.GetCurMoveSpeed` (`self.PropertyComp`)))
  (set `CharacterMovementComponent.MaxWalkSpeed` _returnvalue _charactermovement)
  (set `CharacterMovementComponent.MinAnalogWalkSpeed` 1000.0 _charactermovement))

(event `self.WholeDeath`
  (params (Death :type "Actor Object Reference"))
  (`self.DP_ActorDeath` Death)
  (`self.K2_DestroyActor`))

(fn `UserConstructionScript`)