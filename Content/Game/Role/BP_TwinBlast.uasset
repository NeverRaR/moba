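; TwinBlast hero character that links its PropertyComp stats to movement and the HP/status UI.
; BeginPlay creates the main HUD and sets walk speeds.
; Tick polls PropertyComp to refresh HUD HP, MP, attributes, level and K/D/A, reapply max walk speed, and update the TwinblastHP widget's health ratio with a zero-max guard.
; The EXP percentage is a fixed placeholder, and the Death montage node is never triggered.
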(event `self.ReceiveBeginPlay`
  (bind _charactermovement (`self.CharacterMovement`))
  (`|ExecutionSequence`
    (:`then_0`
      (bind _returnvalue (`|CreateWidget` "/Game/Game/UI/UI_Main.UI_Main_C"))
      (bind _output_get (set `self.MainUI` _returnvalue))
      (`UserWidget.AddToViewport` _output_get 0))
    (:`then_1`
      (bind _returnvalue_2 (`CharacterProperty.GetCurMoveSpeed` (`self.PropertyComp`)))
      (set `CharacterMovementComponent.MaxWalkSpeed` _returnvalue_2 _charactermovement)
      (set `CharacterMovementComponent.MinAnalogWalkSpeed` 1000.0 _charactermovement))))

(event `self.ReceiveTick`
  (params (DeltaSeconds :type "Float (single-precision)"))
  (bind _propertycomp (`self.PropertyComp`))
  (bind _twinblasthp (`self.TwinblastHP`))
  (bind _propertycomp_2 (`self.PropertyComp`))
  (bind _propertycomp_3 (`self.PropertyComp`))
  (bind _mainui (`self.MainUI`))
  (`|ExecutionSequence`
    (:`then_0`
      (`/Engine/EditorBlueprintResources/StandardMacros.IsValid` _mainui
        (:`Is Valid`
          (`|ExecutionSequence`
            (:`then_0`
              (bind _returnvalue (`CharacterProperty.GetCurHP` _propertycomp))
              (bind _returnvalue_2 (`CharacterProperty.GetCurMaxHP` _propertycomp))
              (bind _returnvalue_3 (`CharacterProperty.GetCurHPRecovery` _propertycomp))
              (bind _returnvalue_4 (`CharacterProperty.GetCurMP` _propertycomp))
              (bind _returnvalue_5 (`CharacterProperty.GetCurMaxMP` _propertycomp))
              (bind _returnvalue_6 (`CharacterProperty.GetCurMPRecovery` _propertycomp))
              (`/Game/Game/UI/UI_Main.UpdateStatusHP` _mainui _returnvalue _returnvalue_3 _returnvalue_2)
              (`/Game/Game/UI/UI_Main.UpdateStatusMP` _mainui _returnvalue_4 _returnvalue_5 _returnvalue_6))
            (:`then_1`
              (bind _returnvalue_7 (`CharacterProperty.GetCurPhyAttack` _propertycomp_3))
              (bind _returnvalue_8 (`CharacterProperty.GetCurMagAttack` _propertycomp_3))
              (bind _returnvalue_9 (`CharacterProperty.GetCurPhyDef` _propertycomp_3))
              (bind _returnvalue_10 (`CharacterProperty.GetCurMagDef` _propertycomp_3))
              (bind _returnvalue_11 (`CharacterProperty.GetCurAttackSpeed` _propertycomp_3))
              (bind _returnvalue_12 (`CharacterProperty.GetCurMoveSpeed` _propertycomp_3))
              (bind _returnvalue_13 (`CharacterProperty.GetCurLevel` _propertycomp_3))
              (`CharacterProperty.GetCurEXP` _propertycomp_3)
              (bind _returnvalue_14 (`CharacterProperty.GetCurKillNum` _propertycomp_3))
              (bind _returnvalue_15 (`CharacterProperty.GetCurDeathNum` _propertycomp_3))
              (bind _returnvalue_16 (`CharacterProperty.GetCurAidNum` _propertycomp_3))
              (`/Game/Game/UI/UI_Main.UpdateStatusProperty` _mainui _returnvalue_7 _returnvalue_8 _returnvalue_9 _returnvalue_10 _returnvalue_11 _returnvalue_12 50.0 (`KismetMathLibrary.FTrunc` _returnvalue_13) _returnvalue_14 _returnvalue_15 _returnvalue_16))))))
    (:`then_1`
      (bind _returnvalue_17 (`CharacterProperty.GetCurMoveSpeed` (`self.PropertyComp`)))
      (set `CharacterMovementComponent.MaxWalkSpeed` _returnvalue_17 (`self.CharacterMovement`)))
    (:`then_2`
      (`/Engine/EditorBlueprintResources/StandardMacros.IsValid` _twinblasthp
        (:`Is Valid`
          (`|ExecutionSequence`
            (:`then_0`
              (bind _asui_twinblast (cast `/Game/Game/UI/UI_Twinblast` (`WidgetComponent.GetUserWidgetObject` _twinblasthp)))
              (`/Game/Game/UI/UI_Twinblast.UpdateTwinblastHP` _asui_twinblast (/ (stale _returnvalue_18) (`KismetMathLibrary.SelectFloat` 1.0 (stale _returnvalue_19) (== (stale _returnvalue_19) 0.0)))))
            (:`then_1`
              (bind _returnvalue_18 (`CharacterProperty.GetCurHP` _propertycomp_2))
              (bind _returnvalue_19 (`CharacterProperty.GetCurMaxHP` _propertycomp_2)))))))))

(event `InputAction|LevelUp`
  (params (Key :type "Key Structure")))

(fn `UserConstructionScript`)