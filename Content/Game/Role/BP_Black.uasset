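; BP_Black is a character Blueprint with a property component, an HP bar widget and a minimap sign.
; On BeginPlay it sets walk speed from PropertyComp and fixes a minimum analog walk speed.
; Tick pushes the HP ratio to the UI_Black widget, guarded against zero max HP, before refreshing the cached values, so the bar trails one frame.
; Show and hide events toggle the amber MiniMapSign child actor.
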(event `self.ReceiveBeginPlay`
  (bind _charactermovement (`self.CharacterMovement`))
  (bind _returnvalue (`CharacterProperty.GetCurMoveSpeed` (`self.PropertyComp`)))
  (set `CharacterMovementComponent.MaxWalkSpeed` _returnvalue _charactermovement)
  (set `CharacterMovementComponent.MinAnalogWalkSpeed` 1000.0 _charactermovement))

(event `/Game/Game/Interface/I_MiniMap.ShowMiniMapSign`
  (bind _asmini_map_sign (cast `/Game/Game/MiniMap/MiniMapSign` (`ChildActorComponent.ChildActor` (`self.MiniMapSign`))))
  (`/Game/Game/MiniMap/MiniMapSign.Show Sign` _asmini_map_sign 3.0 null (struct :`R` 1.0 :`G` 0.716867 :`A` 1.0)))

(event `self.DEBUGprint`
  (params (num :type "Float (single-precision)")))

(event `/Game/Game/Interface/I_MiniMap.HiddenMiniMapSign`
  (bind _asmini_map_sign (cast `/Game/Game/MiniMap/MiniMapSign` (`ChildActorComponent.ChildActor` (`self.MiniMapSign`))))
  (`/Game/Game/MiniMap/MiniMapSign.Hidden Sign` _asmini_map_sign))

(event `self.ReceiveTick`
  (params (DeltaSeconds :type "Float (single-precision)"))
  (bind _blackhp (`self.BlackHP`))
  (bind _propertycomp (`self.PropertyComp`))
  (`|ExecutionSequence`
    (:`then_0`
      (`/Engine/EditorBlueprintResources/StandardMacros.IsValid` _blackhp
        (:`Is Valid`
          (`|ExecutionSequence`
            (:`then_0`
              (bind _asui_black (cast `/Game/Game/UI/UI_Black` (`WidgetComponent.GetUserWidgetObject` _blackhp)))
              (`/Game/Game/UI/UI_Black.UpdateBlackHP` _asui_black (/ (stale _returnvalue) (`KismetMathLibrary.SelectFloat` 1.0 (stale _returnvalue_2) (== (stale _returnvalue_2) 0.0)))))
            (:`then_1`
              (bind _returnvalue (`CharacterProperty.GetCurHP` _propertycomp))
              (bind _returnvalue_2 (`CharacterProperty.GetCurMaxHP` _propertycomp)))))))))

(fn `UserConstructionScript`)