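; Player hero Blueprint for Shinbi in a MOBA, linking the character to its HUD and overhead health display.
; BeginPlay retries every 0.2 seconds until the main UI is valid, then sets the hero's head icon.
; InitCamp moves the hero to its camp's start actor, and GameOver forwards the camp to the HUD.
; Tick feeds PropertyComp's health ratio to the ShinbiHP widget; LevelUp input only prints alive status.
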(event `InputAction|LevelUp`
  (params (Key :type "Key Structure"))
  (:`Pressed`
    (bind _returnvalue (`CharacterProperty.IsAlive` (`self.PropertyComp`)))
    (`KismetSystemLibrary.PrintString` (`KismetStringLibrary.Conv_BoolToString` _returnvalue))))

(event `GameOver`
  (params (Camp :type "CharacterCamp Enum" :default "Dawn"))
  (bind _asbp_moba_controller (cast `/Game/Game/Role/BP_MobaController` (`self.GetController`)))
  (bind _asbp_hud (cast `/Game/Game/UI/BP_HUD` (`PlayerController.GetHUD` _asbp_moba_controller)))
  (`/Game/Game/UI/BP_HUD.OnGameOver` _asbp_hud Camp))

(event `self.ReceiveBeginPlay`
  (`|ExecutionSequence`
    (:`then_0`
      (bind _asbp_moba_controller (cast `/Game/Game/Role/BP_MobaController` (`self.GetController`)))
      (bind _asbp_hud (cast `/Game/Game/UI/BP_HUD` (`PlayerController.GetHUD` _asbp_moba_controller)))
      (bind _mainui (`/Game/Game/UI/BP_HUD.MainUI` _asbp_hud))
      (`/Engine/EditorBlueprintResources/StandardMacros.IsValid` _mainui :!label _label
        (:`Is Valid`
          (`Image.SetBrushFromTexture` (`/Game/Game/UI/UI_Status_Property.HeadIcon` (`/Game/Game/UI/UI_Main.UI_Status_Property` _mainui)) "/Game/Game/TextureAndMat/UI/HeadIcon.HeadIcon" true))
        (:`Is Not Valid`
          (`KismetSystemLibrary.Delay` 0.2)
          (goto _label))))))

(event `InitCamp`
  (bind _returnvalue (`CreatureCamp.GetCamp` (`self.CampComp`)))
  (switch `CharacterCamp` _returnvalue
    (:`Dawn`
      (bind _outactors (`GameplayStatics.GetAllActorsOfClass` "/Game/Game/Dawn/DawnBeginPlayer.DawnBeginPlayer_C"))
      (bind _output (`|GetArrayItem` _outactors))
      (`/Engine/EditorBlueprintResources/StandardMacros.IsValid` _output
        (:`Is Valid`
          (set `self.OriginLocation` (`self.K2_GetActorLocation` _output)))))
    (:`Dust`
      (bind _outactors_2 (`GameplayStatics.GetAllActorsOfClass` "/Game/Game/Dusk/DuskBeginPlayer.DuskBeginPlayer_C"))
      (bind _output_2 (`|GetArrayItem` _outactors_2))
      (`/Engine/EditorBlueprintResources/StandardMacros.IsValid` _output_2
        (:`Is Valid`
          (set `self.OriginLocation` (`self.K2_GetActorLocation` _output_2))))))
  (`self.K2_SetActorLocation` (`self.OriginLocation`)))

(event `self.ReceiveTick`
  (params (DeltaSeconds :type "Float (single-precision)"))
  (bind _propertycomp (`self.PropertyComp`))
  (bind _shinbihp (`self.ShinbiHP`))
  (`|ExecutionSequence`
    (:`then_0`
      (`/Engine/EditorBlueprintResources/StandardMacros.IsValid` _shinbihp
        (:`Is Valid`
          (`|ExecutionSequence`
            (:`then_0`
              (bind _asui_shinbi (cast `/Game/Game/UI/UI_Shinbi` (`WidgetComponent.GetUserWidgetObject` _shinbihp)))
              (`/Game/Game/UI/UI_Shinbi.UpdateShinbiHP` _asui_shinbi (/ (stale _returnvalue) (`KismetMathLibrary.SelectFloat` 1.0 (stale _returnvalue_2) (== (stale _returnvalue_2) 0.0)))))
            (:`then_1`
              (bind _returnvalue (`CharacterProperty.GetCurHP` _propertycomp))
              (bind _returnvalue_2 (`CharacterProperty.GetCurMaxHP` _propertycomp)))))))))

(fn `UserConstructionScript`)