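; BP_Minion_Ranged is a ranged minion character that exposes events for movement speed, death and firing effects.
; SetFireParticle passes an emitter to MulticastPlayEffects to spawn at the Muzzle_Front socket, while WholeDeath calls CallDPActorDeath and destroys the actor.
; Tick feeds the HP ratio to the UI_Minion_Ranged widget with a zero-max guard, then refreshes cached HP from PropertyComp, so the bar uses the previous tick's values.
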(event `MulticastPlayEffects`
  (params (Emitter :type "ParticleSystem Object Reference") (Location :type "Vector Structure") (Rotation :type "Rotator Structure"))
  (`GameplayStatics.SpawnEmitterAtLocation` Emitter Location Rotation))

(event `self.SetMoveSpeed`
  (params (CurSpeed :type "Float (single-precision)"))
  (bind _charactermovement (`self.CharacterMovement`))
  (set `CharacterMovementComponent.MaxWalkSpeed` CurSpeed _charactermovement)
  (set `CharacterMovementComponent.MinAnalogWalkSpeed` 1000.0 _charactermovement))

(event `self.WholeDeath`
  (params (Death :type "Actor Object Reference"))
  (`self.DP_ActorDeath` Death)
  (`self.K2_DestroyActor`))

(event `self.SetFireParticle`
  (params (React :type "ParticleSystem Object Reference") (Combo :type Integer))
  (`self.MulticastPlayEffects` React (`SceneComponent.GetSocketLocation` (`self.Mesh`) "Muzzle_Front") (`self.K2_GetActorRotation`)))

(event `self.CDelay`
  (params (time :type "Float (single-precision)"))
  (`KismetSystemLibrary.Delay` time))

(event `self.ReceiveTick`
  (params (DeltaSeconds :type "Float (single-precision)"))
  (bind _propertycomp (`self.PropertyComp`))
  (bind _hp (`self.HP`))
  (`|ExecutionSequence`
    (:`then_0`
      (`/Engine/EditorBlueprintResources/StandardMacros.IsValid` _hp
        (:`Is Valid`
          (`|ExecutionSequence`
            (:`then_0`
              (bind _asui_minion_ranged (cast `/Game/Game/UI/UI_Minion_Ranged` (`WidgetComponent.GetUserWidgetObject` _hp)))
              (`/Game/Game/UI/UI_Minion_Ranged.UpdateMinionRangedHP` _asui_minion_ranged (/ (stale _returnvalue) (`KismetMathLibrary.SelectFloat` 1.0 (stale _returnvalue_2) (== (stale _returnvalue_2) 0.0)))))
            (:`then_1`
              (bind _returnvalue (`CharacterProperty.GetCurHP` _propertycomp))
              (bind _returnvalue_2 (`CharacterProperty.GetCurMaxHP` _propertycomp)))))))))

(fn `UserConstructionScript`)