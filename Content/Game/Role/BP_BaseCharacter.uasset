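; Base character Blueprint that pairs a PropertyComp stat component with a main HUD and level-up testing.
; BeginPlay overrides physical attack and creates UI_Main, which Tick refreshes by polling the component for HP, MP, combat stats and level.
; LevelUp input or K runs a level-up check and prints base stats; other debug keys call AddEXP and print nearby enemy counts.
; SetMoveSpeed applies walk speed to CharacterMovement.
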(event `self.ReceiveBeginPlay`
  (`|ExecutionSequence`
    (:`then_0`
      (`/Engine/EditorBlueprintResources/StandardMacros.IsValid` null
        (:`Is Valid`
          (`|ExecutionSequence`
            (:`then_1`
              (`CharacterProperty.SetCurPhyAttack` (`self.PropertyComp`) 150.0))))))
    (:`then_1`
      (bind _returnvalue (`|CreateWidget` "/Game/Game/UI/UI_Main.UI_Main_C"))
      (bind _output_get (set `self.MainUI` _returnvalue))
      (`UserWidget.AddToViewport` _output_get 0))))

(event `self.SetMoveSpeed`
  (params (CurSpeed :type "Float (single-precision)"))
  (bind _charactermovement (`self.CharacterMovement`))
  (set `CharacterMovementComponent.MaxWalkSpeed` CurSpeed _charactermovement)
  (set `CharacterMovementComponent.MinAnalogWalkSpeed` 1000.0 _charactermovement))

(event `InputAction|LevelUp`
  (params (Key :type "Key Structure"))
  (bind _propertycomp (`self.PropertyComp`))
  (:`Pressed`
    (bind _returnvalue (`self.GetAllEnemysInRadius` 2000.0 :!label _label))
    (`KismetSystemLibrary.PrintString` (`KismetStringLibrary.Conv_IntToString` (`KismetArrayLibrary.Array_Length` _returnvalue)))
    (`CharacterProperty.CheckLevelUp` _propertycomp 100.0)
    (bind _returnvalue_2 (`CharacterProperty.GetCurLevel` _propertycomp))
    (bind _returnvalue_3 (`CharacterProperty.GetBaseMaxHP` _propertycomp))
    (bind _returnvalue_4 (`CharacterProperty.GetBaseMaxMP` _propertycomp))
    (bind _returnvalue_5 (`CharacterProperty.GetBaseMPRecovery` _propertycomp))
    (bind _returnvalue_6 (`CharacterProperty.GetBaseHPRecovery` _propertycomp))
    (bind _returnvalue_7 (`CharacterProperty.GetBasePhyAttack` _propertycomp))
    (bind _returnvalue_8 (`CharacterProperty.GetBaseMagAttack` _propertycomp))
    (`KismetSystemLibrary.PrintString` (`KismetStringLibrary.Concat_StrStr` "HP " (`KismetStringLibrary.Conv_DoubleToString` _returnvalue_3) " MP " (`KismetStringLibrary.Conv_DoubleToString` _returnvalue_4) " HPRecovery  " (`KismetStringLibrary.Conv_DoubleToString` _returnvalue_5) " HPRecovery  " (`KismetStringLibrary.Conv_DoubleToString` _returnvalue_6) " PhyAttack " (`KismetStringLibrary.Conv_DoubleToString` _returnvalue_7) " MagAttack " (`KismetStringLibrary.Conv_DoubleToString` _returnvalue_8) " Level " (`KismetStringLibrary.Conv_DoubleToString` _returnvalue_2)) true true (struct :`G` 0.66 :`B` 1.0 :`A` 1.0) 600.0)))

(event `self.DEBUGprint`
  (params (num :type "Float (single-precision)"))
  (`KismetSystemLibrary.PrintString` (`KismetStringLibrary.Conv_DoubleToString` num)))

(event `Key|K`
  (params (Key :type "Key Structure"))
  (:`Pressed`
    (goto _label)))

(event `self.ReceiveTick`
  (params (DeltaSeconds :type "Float (single-precision)"))
  (bind _propertycomp (`self.PropertyComp`))
  (bind _propertycomp_2 (`self.PropertyComp`))
  (bind _mainui (`self.MainUI`))
  (`|ExecutionSequence`
    (:`then_0`
      (`/Engine/EditorBlueprintResources/StandardMacros.IsValid` _mainui
        (:`Is Valid`
          (`|ExecutionSequence`
            (:`then_0`
              (`/Game/Game/UI/UI_Main.UpdateStatusHP` _mainui (stale _returnvalue) (stale _returnvalue_3) (stale _returnvalue_2))
              (`/Game/Game/UI/UI_Main.UpdateStatusMP` _mainui (stale _returnvalue_4) (stale _returnvalue_5) (stale _returnvalue_6))
              (bind _returnvalue (`CharacterProperty.GetCurHP` _propertycomp))
              (bind _returnvalue_2 (`CharacterProperty.GetCurMaxHP` _propertycomp))
              (bind _returnvalue_3 (`CharacterProperty.GetBaseHPRecovery` _propertycomp))
              (bind _returnvalue_4 (`CharacterProperty.GetCurMP` _propertycomp))
              (bind _returnvalue_5 (`CharacterProperty.GetCurMaxMP` _propertycomp))
              (bind _returnvalue_6 (`CharacterProperty.GetBaseMPRecovery` _propertycomp)))
            (:`then_1`
              (`/Game/Game/UI/UI_Main.UpdateStatusProperty` _mainui (stale _returnvalue_7) (stale _returnvalue_8) (stale _returnvalue_9) (stale _returnvalue_10) (stale _returnvalue_11) (stale _returnvalue_12) 0.0 (`KismetMathLibrary.FTrunc` (stale _returnvalue_13)) 0.0 0.0 0.0)
              (bind _returnvalue_7 (`CharacterProperty.GetCurPhyAttack` _propertycomp_2))
              (bind _returnvalue_8 (`CharacterProperty.GetCurMagAttack` _propertycomp_2))
              (bind _returnvalue_9 (`CharacterProperty.GetCurPhyDef` _propertycomp_2))
              (bind _returnvalue_10 (`CharacterProperty.GetCurMagDef` _propertycomp_2))
              (bind _returnvalue_11 (`CharacterProperty.GetCurAttackSpeed` _propertycomp_2))
              (bind _returnvalue_12 (`CharacterProperty.GetCurMoveSpeed` _propertycomp_2))
              (`CharacterProperty.GetCurEXP` _propertycomp_2)
              (bind _returnvalue_13 (`CharacterProperty.GetCurLevel` _propertycomp_2)))
            (:`then_2`
              (bind _returnvalue_14 (`self.GetAllEnemysInRadius` self 500.0)))))))))

(event `Key|One`
  (params (Key :type "Key Structure"))
  (:`Pressed`
    (`CharacterProperty.AddEXP` (`self.PropertyComp`) 0.0)))

(event `Key|Two`
  (params (Key :type "Key Structure"))
  (:`Pressed`
    (`KismetSystemLibrary.PrintString` (`KismetStringLibrary.Conv_IntToString` (`KismetArrayLibrary.Array_Length` (stale `self.ReceiveTick` _returnvalue_14))))))

(fn `UserConstructionScript`)