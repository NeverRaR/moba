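; Turret character Blueprint that aims at its AI-chosen attack target and shows targeting effects.
; Each tick it reads the Blackboard target, moves a focus point toward it at constant speed to drive the anim Blueprint's look-at, and sets ReadyAttack once close.
; Range checks toggle the beam, while a muzzle line trace binds it to the target.
; Events also handle muzzle particles, walk speed and death.
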(event `self.DEBUGprint`
  (params (num :type "Float (single-precision)")))

(event `self.SetFireParticle`
  (params (React :type "ParticleSystem Object Reference"))
  (`GameplayStatics.SpawnEmitterAtLocation` React (`SceneComponent.GetSocketLocation` (`self.Mesh`) "Muzzle_01") (`self.K2_GetActorRotation`)))

(event `self.SetMoveSpeed`
  (params (CurSpeed :type "Float (single-precision)"))
  (bind _charactermovement (`self.CharacterMovement`))
  (set `CharacterMovementComponent.MaxWalkSpeed` CurSpeed _charactermovement)
  (set `CharacterMovementComponent.MinAnalogWalkSpeed` 1000.0 _charactermovement))

(event `self.WholeDeath`
  (params (Death :type "Actor Object Reference"))
  (`self.DP_ActorDeath` Death)
  (`self.K2_DestroyActor`))

(event `self.ReceiveTick`
  (params (DeltaSeconds :type "Float (single-precision)"))
  (bind _returnvalue (`AIBlueprintHelperLibrary.GetBlackboard` (`self.GetController`)))
  (bind _returnvalue_2 (`BlackboardComponent.GetValueAsBool` _returnvalue "IsCombat"))
  (bind _returnvalue_3 (`BlackboardComponent.GetValueAsObject` _returnvalue "AttackTarget"))
  (`|ExecutionSequence`
    (:`then_0`
      (bind _asabp_turret (cast `/Game/Game/Animation/ABP_Turret` (`SkeletalMeshComponent.GetAnimInstance` (`self.Mesh`))))
      (`/Engine/EditorBlueprintResources/StandardMacros.IsValid` _returnvalue_3
        (:`Is Valid`
          (set `self.TargetLocation` (`BlackboardComponent.GetValueAsVector` _returnvalue "AttackTargetLocation"))
          (bind _output_get (set `self.FocusLocation` (`KismetMathLibrary.VInterpTo_Constant` (`self.FocusLocation`) (`self.TargetLocation`) (`GameplayStatics.GetWorldDeltaSeconds`) 1200.0)))
          (set `/Game/Game/Animation/ABP_Turret.IsCombat` _returnvalue_2 _asabp_turret)
          (set `/Game/Game/Animation/ABP_Turret.LookAtLotation` _output_get _asabp_turret)
          (bind _returnvalue_4 (`CharacterProperty.GetAttackRange` (`self.PropertyComp`)))
          (if (>= (- _returnvalue_4 -100.0) (`BlackboardComponent.GetValueAsFloat` _returnvalue "DistanceToTarget"))
            (`SceneComponent.SetVisibility` (`self.TargetBeam`) true false)
            (`SceneComponent.SetVisibility` (`self.TargetSign`) true false)
            (`SceneComponent.K2_SetWorldLocation` (`self.TargetSign`) (`self.TargetLocation`) false false)
            (else
              (`SceneComponent.SetVisibility` (`self.TargetBeam`) false true :!label _label)
              (set `/Game/Game/Animation/ABP_Turret.IsCombat` _returnvalue_2 _asabp_turret))))
        (:`Is Not Valid`
          (goto _label))))
    (:`then_1`
      (set `self.ReadyAttack` (<= (`KismetMathLibrary.VSize` (- (`self.TargetLocation`) (`self.FocusLocation`))) 100.0)))
    (:`then_2`
      (`/Engine/EditorBlueprintResources/StandardMacros.IsValid` _returnvalue_3
        (:`Is Valid`
          (bind _asactor (cast `Actor` _returnvalue_3))
          (bind (_outhits _returnvalue_5) (`KismetSystemLibrary.LineTraceMultiForObjects` (`SceneComponent.GetSocketLocation` (`self.Mesh`) "Muzzle_01") (`self.K2_GetActorLocation` _asactor) (`|MakeArray` "ObjectTypeQuery3" :!type "EObjectTypeQuery Enum")))
          (if _returnvalue_5
            (for _array_element _outhits
              (bind (_bblockinghit _binitialoverlap _time _distance _location _impactpoint _normal _impactnormal _physmat _hitactor) (`GameplayStatics.BreakHitResult` _array_element))
              (if (== _hitactor _asactor)
                (`ParticleSystemComponent.SetActorParameter` (`self.TargetBeam`) "Target" _hitactor)))))))))

(fn `UserConstructionScript`)